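; RTS player controller that handles mouse input for marquee selection and unit move orders, with a visible cursor locked to the viewport.
; Left mouse press, hold (polled on Tick) and release are forwarded to the HUD as marquee messages.
; Right click traces under the cursor, sends a move command to every selected unit fetched from the HUD, and spawns a cursor effect at that location.
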(event `self.ReceiveBeginPlay`
  (`WidgetBlueprintLibrary.SetInputMode_GameAndUIEx` self null "LockAlways" false)
  (set `self.bShowMouseCursor` true))

(event `self.ReceiveTick`
  (params (DeltaSeconds :type "Float (single-precision)"))
  (if (`self.bIsLeftMousePressed`)
    (message `/Game/Blueprints/BPI_RTS_Interface.MarqueeHeld` (`self.GetHUD`))))

(event `Key|LeftMouseButton`
  (params (Key :type "Key Structure"))
  (bind _returnvalue (`self.GetHUD`))
  (:`Pressed`
    (set `self.bIsLeftMousePressed` true)
    (message `/Game/Blueprints/BPI_RTS_Interface.MarqueePressed` _returnvalue))
  (:`Released`
    (set `self.bIsLeftMousePressed` false)
    (message `/Game/Blueprints/BPI_RTS_Interface.MarqueeReleased` _returnvalue)))

(event `Key|RightMouseButton`
  (params (Key :type "Key Structure"))
  (:`Pressed`
    (set `self.RightClickLocation` (`.Location` (`GameplayStatics.BreakHitResult` (`self.GetHitResultUnderCursorByChannel` "TraceTypeQuery1"))))
    (bind _units (message `/Game/Blueprints/BPI_RTS_Interface.GrabSelectedUnits` (`self.GetHUD`)))
    (for _array_element _units
      (message `/Game/Blueprints/BPI_RTS_Interface.UnitMoveCommand` _array_element (`self.RightClickLocation`)))
    (`NiagaraFunctionLibrary.SpawnSystemAtLocation` "/Game/Cursor/FX_Cursor.FX_Cursor" (`self.RightClickLocation`))))

(fn `GrabSelectedUnits`
  (returns (Units :type "Array of Actor Object Reference"))
  (return))

(fn `UserConstructionScript`)