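; BP_CameraPawn is a camera pawn that pans across the world by edge scrolling when the mouse nears the screen border.
; MouseX and MouseY axis events divide the cursor position by the viewport size and test it against thin margins at each edge.
; Inside a margin, the pawn offsets along world Y (horizontal edges) or X (vertical edges) by ScrollSpeed scaled by delta time.
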(event `InputAxisKey|MouseX`
  (params (AxisValue :type "Float (single-precision)"))
  (bind _returnvalue_x (`KismetMathLibrary.BreakVector2D` (`WidgetLayoutLibrary.GetViewportSize`)))
  (bind _returnvalue (/ (`PlayerController.GetMousePosition` (`GameplayStatics.GetPlayerController` 0)) _returnvalue_x))
  ; Edge Scrolling
  (if (> _returnvalue 0.98)
    (`self.K2_AddActorWorldOffset` (`KismetMathLibrary.MakeVector` 0.0 (* (`self.ScrollSpeed`) (`GameplayStatics.GetWorldDeltaSeconds`))))
    (elif (< _returnvalue 0.02)
      (`self.K2_AddActorWorldOffset` (`KismetMathLibrary.MakeVector` 0.0 (* (* (`self.ScrollSpeed`) (`GameplayStatics.GetWorldDeltaSeconds`)) -1.0))))))

(event `InputAxisKey|MouseY`
  (params (AxisValue :type "Float (single-precision)"))
  (bind (_returnvalue_x _returnvalue_y) (`KismetMathLibrary.BreakVector2D` (`WidgetLayoutLibrary.GetViewportSize`)))
  (bind _returnvalue (/ (`.LocationY` (`PlayerController.GetMousePosition` (`GameplayStatics.GetPlayerController` 0))) _returnvalue_y))
  ; Edge Scrolling
  (if (> _returnvalue 0.98)
    (`self.K2_AddActorWorldOffset` (`KismetMathLibrary.MakeVector` (* (* (`self.ScrollSpeed`) (`GameplayStatics.GetWorldDeltaSeconds`)) -1.0)))
    (elif (< _returnvalue 0.02)
      (`self.K2_AddActorWorldOffset` (`KismetMathLibrary.MakeVector` (* (`self.ScrollSpeed`) (`GameplayStatics.GetWorldDeltaSeconds`)))))))

(fn `UserConstructionScript`)