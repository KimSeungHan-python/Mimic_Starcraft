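; Base RTS building that queues and produces units for its team, with a selection decal and command widget.
; BeginPlay builds the widget from action buttons and tints mesh and minimap materials through dynamic TeamColor instances.
; A looping server-only timer pulls queued unit classes and spawns them with team data once progress reaches 0.1 of their ProductionTime.
; Server overlaps send DropOffMessage to the other actor; interface-style functions besides GetTeam are stubs.
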(event `self.ReceiveActorBeginOverlap`
  (params (OtherActor :type "Actor Object Reference"))
  (`/Engine/EditorBlueprintResources/ActorMacros.Switch Has Authority`
    (:`Authority`
      (message `/Game/Blueprints/RTS/BPI_RTSResource.DropOff` OtherActor))))

(event `AddUnitToQueue`
  (params (Unit :type "/Game/Blueprints/RTS/Units/BP_Unit_Base Class Reference"))
  (`KismetArrayLibrary.Array_Add` (`self.UnitProductcionQueue`) Unit))

(event `/Game/Blueprints/RTS/BPI_RTS_Interface.SelectedThis_Decal`
  (`SceneComponent.SetVisibility` (`self.Decal`) true false)
  (`UserWidget.AddToViewport` (`self.WBPClickedBuilding`) 0))

(event `/Game/Blueprints/RTS/BPI_RTS_Interface.DeselectedThis_Decal`
  (`SceneComponent.SetVisibility` (`self.Decal`) false false)
  (`Widget.RemoveFromParent` (`self.WBPClickedBuilding`)))

(event `self.ReceiveBeginPlay`
  (`|ExecutionSequence`
    (:`then_0`
      ; Create Building Widget
      (bind _returnvalue (`|CreateWidget` "/Game/Blueprints/WBP_ClickedBuilding.WBP_ClickedBuilding_C"))
      (set `self.WBPClickedBuilding` _returnvalue)
      (set `/Game/Blueprints/WBP_ClickedBuilding.Building_Base` self _returnvalue)
      (for _array_element (`self.ActionBoxButtons`)
        (`WrapBox.AddChildToWrapBox` (`/Game/Blueprints/WBP_ClickedBuilding.ActionBox` (`self.WBPClickedBuilding`)) _array_element)))
    (:`then_1`
      ; Setup TeamColor
      (for (_array_element_2 _array_index) (`MeshComponent.GetMaterials` (`self.Mesh`))
        (bind _returnvalue_2 (`KismetMaterialLibrary.CreateDynamicMaterialInstance` _array_element_2))
        (`MaterialInstanceDynamic.SetVectorParameterValue` _returnvalue_2 "TeamColor" (`self.TeamColor`))
        (`PrimitiveComponent.SetMaterial` (`self.Mesh`) _array_index _returnvalue_2))
      (bind _returnvalue_3 (`KismetMaterialLibrary.CreateDynamicMaterialInstance` (`PrimitiveComponent.GetMaterial` (`self.SMC_MiniMap`) 0)))
      (`MaterialInstanceDynamic.SetVectorParameterValue` _returnvalue_3 "TeamColor" (`self.TeamColor`))
      (`PrimitiveComponent.SetMaterial` (`self.SMC_MiniMap`) 0 _returnvalue_3))
    (:`then_2`
      (`/Engine/EditorBlueprintResources/ActorMacros.Switch Has Authority`
        (:`Authority`
          (`KismetSystemLibrary.K2_SetTimerDelegate` (delegate `ProcessProductionQueue`) (`self.ProductionTimerGranluarity`) true))))))

(event `ProcessProductionQueue`
  (if (`self.bIsProdcucingUnit`)
    (bind _output_get (set `self.Production TimeSpent` (+ (`self.Production TimeSpent`) (`self.ProductionTimerGranluarity`))))
    (bind _output_get_2 (set `self.Production Progress` (/ _output_get (`self.Production TimeNeeded`))))
    (if (>= _output_get_2 0.1)
      (`|SpawnActorFromClass` (`self.UnitBeingProducing`) (`KismetMathLibrary.MakeTransform` (`SceneComponent.K2_GetComponentLocation` (`self.UnitSpawnPoints`))) "AdjustIfPossibleButAlwaysSpawn" "MultiplyWithRoot" null (`self.TeamColor`) (`self.TeamNumber`) null)
      (set `self.Production TimeSpent` 0.0)
      (set `self.Production Progress` 0.0)
      (set `self.bIsProdcucingUnit` false)
      (set `self.UnitBeingProducing` null))
    (elif (> (`KismetArrayLibrary.Array_Length` (`self.UnitProductcionQueue`)) 0)
      (bind _output_get_3 (set `self.UnitBeingProducing` (`|GetArrayItem` (`self.UnitProductcionQueue`))))
      (set `self.Production TimeNeeded` (`.ProductionTime` (defaults `Object` _output_get_3)))
      (`KismetArrayLibrary.Array_Remove` (`self.UnitProductcionQueue`))
      (set `self.bIsProdcucingUnit` true))))

(fn `GetResources`
  (returns (Amounts :type Integer))
  (return 0))

(fn `GetTeam`
  (returns (TeamNumber :type Integer))
  (return (`self.TeamNumber`)))

(fn `GrabSelectedUnits`
  (returns (Units :type "Array of Actor Object Reference"))
  (return))

(fn `IsOnMyTeam`
  (params (TeamNumber :type Integer))
  (returns (MyTeam :type Boolean))
  (return false))

(fn `UserConstructionScript`)