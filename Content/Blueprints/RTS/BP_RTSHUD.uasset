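; RTS HUD that handles marquee drag-selection of units and holds the selected unit list.
; Marquee events track mouse corners while DrawHUD draws the translucent box, gathers BP_Unit_Base actors inside, selects those on the player's team and clears the controller's building selection.
; Units outside the box are deselected unless the controller's LeftShift is set.
; Events for single-select and clear, plus a getter, expose the list; team functions return fixed defaults.
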(event `/Game/Blueprints/RTS/BPI_RTS_Interface.MarqueePressed`
  (bind (_locationx _locationy) (`PlayerController.GetMousePosition` (`GameplayStatics.GetPlayerController` 0)))
  ; Marquee Start
  (set `self.bIsDrawing` true)
  (bind _output_get (set `self.StartMousePosition` (`KismetMathLibrary.MakeVector2D` _locationx _locationy)))
  (set `self.CurrentMousePosition` _output_get))

(event `/Game/Blueprints/RTS/BPI_RTS_Interface.MarqueeHeld`
  (bind (_locationx _locationy) (`PlayerController.GetMousePosition` (`GameplayStatics.GetPlayerController` 0)))
  ; Marquee Held
  (set `self.CurrentMousePosition` (`KismetMathLibrary.MakeVector2D` _locationx _locationy)))

(event `/Game/Blueprints/RTS/BPI_RTS_Interface.MarqueeReleased`
  ; Marquee Released
  (set `self.bIsDrawing` false))

(event `self.ReceiveDrawHUD`
  (params (SizeX :type Integer) (SizeY :type Integer))
  (bind (_startmouseposition_x _startmouseposition_y) (`KismetMathLibrary.BreakVector2D` (`self.StartMousePosition`)))
  (bind (_currentmouseposition_x _currentmouseposition_y) (`KismetMathLibrary.BreakVector2D` (`self.CurrentMousePosition`)))
  (bind (_startmouseposition_x_2 _startmouseposition_y_2) (`KismetMathLibrary.BreakVector2D` (`self.StartMousePosition`)))
  (if (`self.bIsDrawing`)
    (`self.DrawRect` (struct :`R` 0.060954 :`G` 1.0 :`B` 0.034783 :`A` 0.2) _startmouseposition_x _startmouseposition_y (- _currentmouseposition_x _startmouseposition_x_2) (- _currentmouseposition_y _startmouseposition_y_2))
    (bind _output_get (set `self.ActorInRectangle` (`self.GetActorsInSelectionRectangle` "/Game/Blueprints/RTS/Units/BP_Unit_Base.BP_Unit_Base_C" (`self.StartMousePosition`) (`self.CurrentMousePosition`) false)))
    (for _array_element _output_get
      ; Selecting Units
      (bind _teamnumber (message `/Game/Blueprints/RTS/BPI_RTS_Interface.GetTeam` _array_element))
      (bind _myteam (message `/Game/Blueprints/RTS/BPI_RTS_Interface.IsOnMyTeam` (`GameplayStatics.GetPlayerController` 0) _teamnumber))
      (if _myteam
        (message `/Game/Blueprints/RTS/BPI_RTS_Interface.SelectedThis_Decal` _array_element)
        (`KismetArrayLibrary.Array_AddUnique` (`self.SelectedUnits`) _array_element)
        (message `/Game/Blueprints/RTS/BPI_RTS_Interface.ClearSelectedBuildings` (`GameplayStatics.GetPlayerController` 0))))
    ; Select Units
    (for _array_element_2 (`self.SelectedUnits`)
      (if (== (`KismetArrayLibrary.Array_Find` (`self.ActorInRectangle`) _array_element_2) -1)
        (bind _asbp_rtsplayer_controller (cast `/Game/Blueprints/RTS/BP_RTSPlayerController` (`GameplayStatics.GetPlayerController` 0)))
        (if (not (`/Game/Blueprints/RTS/BP_RTSPlayerController.LeftShift` _asbp_rtsplayer_controller))
          (message `/Game/Blueprints/RTS/BPI_RTS_Interface.DeselectedThis_Decal` _array_element_2)
          (`KismetArrayLibrary.Array_RemoveItem` (`self.SelectedUnits`) _array_element_2))))))

(event `/Game/Blueprints/RTS/BPI_RTS_Interface.ClearSelectedUnits`
  (bind _selectedunits (`self.SelectedUnits`))
  ; Clear Selected Units
  (for _array_element _selectedunits
    (message `/Game/Blueprints/RTS/BPI_RTS_Interface.DeselectedThis_Decal` _array_element))
  (`KismetArrayLibrary.Array_Clear` _selectedunits))

(event `/Game/Blueprints/RTS/BPI_RTS_Interface.SelectSingleUnit`
  (params (Unit :type "Actor Object Reference"))
  ; Select Single Unit
  (message `/Game/Blueprints/RTS/BPI_RTS_Interface.SelectedThis_Decal` Unit)
  (`KismetArrayLibrary.Array_AddUnique` (`self.SelectedUnits`) Unit))

(fn `GetTeam`
  (returns (TeamNumber :type Integer))
  (return 0))

(fn `GrabSelectedUnits`
  (returns (Units :type "Array of Actor Object Reference"))
  (return (`self.SelectedUnits`)))

(fn `IsOnMyTeam`
  (params (TeamNumber :type Integer))
  (returns (MyTeam :type Boolean))
  (return false))

(fn `UserConstructionScript`)