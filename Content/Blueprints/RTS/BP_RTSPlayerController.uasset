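; Player controller for the RTS mode, handling selection, unit orders, resources, unit production and the team's starting spawn.
; Left click selects an own-team building and drives the HUD marquee; right click sends selected units to move or work resource nodes through S2C events.
; Production requests check and deduct unit price before queuing, while authority-only setup spawns a starting building and two resource units.
; Local BeginPlay creates the units widget and aligns its minimap to camera yaw.
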(event `/Game/Blueprints/RTS/BPI_RTS_Interface.IncrementResourceAmout`
  (params (ResourceAmount :type Integer))
  ; Increment Resource Amounts
  (set `self.ResoureceAmounts` (+ ResourceAmount (`self.ResoureceAmounts`))))

(event `S2CAddUnitToQueue`
  (params (Building :type "/Game/Blueprints/RTS/BP_Building_Base Object Reference") (Unit :type "/Game/Blueprints/RTS/Units/BP_Unit_Base Class Reference"))
  (bind (_2d_image _teamcolor _teamnumber _productiontime _unitprice) (defaults `Object` Unit))
  (if (> (`self.ResoureceAmounts`) _unitprice)
    (set `self.ResoureceAmounts` (- (`self.ResoureceAmounts`) _unitprice))
    (`/Game/Blueprints/RTS/BP_Building_Base.AddUnitToQueue` Building Unit)
    (else
      (`self.S2OwnC_ShowNotEnoughResources`))))

(event `S2OwnC_ShowNotEnoughResources`
  (`/Game/Blueprints/RTS/WBP_Units.ShowNotEnoughResourcesMessage` (`self.WBPUnitsRef`)))

(event `/Game/Blueprints/RTS/BPI_RTS_Interface.ProduceUnit`
  (params (Building :type "/Game/Blueprints/RTS/BP_Building_Base Object Reference") (Unit :type "/Game/Blueprints/RTS/Units/BP_Unit_Base Class Reference"))
  (`self.S2CAddUnitToQueue` Building Unit))

(event `/Game/Blueprints/RTS/BPI_RTS_Interface.SetupPlayerStart`
  (params (PlayerStartCamp :type "/Game/Blueprints/BP_PlayerStartCamp Object Reference") (TeamNumber :type Integer) (TemColor :type "LinearColor Structure"))
  ; 서버만 권한
  (`/Engine/EditorBlueprintResources/ActorMacros.Switch Has Authority`
    (:`Authority`
      (set `self.Team Number` TeamNumber)
      (set `self.Tem Color` TemColor)
      (`self.SetupStart` PlayerStartCamp))))

(event `/Game/Blueprints/RTS/BPI_RTS_Interface.ClearSelectedBuildings`
  (bind _selectedbuilding (`self.SelectedBuilding`))
  ; ClearBuilding
  (`/Engine/EditorBlueprintResources/StandardMacros.IsValid` _selectedbuilding
    (:`Is Valid`
      (message `/Game/Blueprints/RTS/BPI_RTS_Interface.DeselectedThis_Decal` _selectedbuilding)
      (set `self.SelectedBuilding` null))))

(event `/Game/Blueprints/RTS/BPI_RTS_Interface.AddUnitToSelectedUnits`
  (params (Widget :type "UserWidget Object Reference"))
  (`HorizontalBox.AddChildToHorizontalBox` (`/Game/Blueprints/RTS/WBP_Units.UnitsBox` (`self.WBPUnitsRef`)) Widget))

(event `self.ReceiveBeginPlay`
  (bind (_returnvalue_roll _returnvalue_pitch _returnvalue_yaw) (`KismetMathLibrary.BreakRotator` (`SceneComponent.K2_GetComponentRotation` (`PlayerCameraManager.TransformComponent` (`GameplayStatics.GetPlayerCameraManager` 0)))))
  (if (`self.IsLocalPlayerController`)
    (`WidgetBlueprintLibrary.SetInputMode_GameAndUIEx` self null "LockAlways" false)
    (set `self.bShowMouseCursor` true)
    (bind _returnvalue (`|CreateWidget` "/Game/Blueprints/RTS/WBP_Units.WBP_Units_C"))
    (bind _output_get (set `self.WBPUnitsRef` _returnvalue))
    (`UserWidget.AddToViewport` _output_get 0)
    (`Widget.SetRenderTransformAngle` (`/Game/Blueprints/RTS/WBP_Units.Overlay_Minimap` _returnvalue) _returnvalue_yaw)))

(event `self.ReceiveTick`
  (params (DeltaSeconds :type "Float (single-precision)"))
  (if (`self.bIsLeftMousePressed`)
    (message `/Game/Blueprints/RTS/BPI_RTS_Interface.MarqueeHeld` (`self.GetHUD`))))

(event `Key|LeftMouseButton`
  (params (Key :type "Key Structure"))
  (bind _returnvalue (`self.GetHUD`))
  (bind _bisinbuildmode (`self.bIsInBuildMode`))
  (:`Pressed`
    (if (not _bisinbuildmode)
      (set `self.bIsLeftMousePressed` true)
      (`self.SelectBuilding`)
      (message `/Game/Blueprints/RTS/BPI_RTS_Interface.MarqueePressed` _returnvalue)))
  (:`Released`
    (if (not _bisinbuildmode)
      (set `self.bIsLeftMousePressed` false)
      (message `/Game/Blueprints/RTS/BPI_RTS_Interface.MarqueeReleased` _returnvalue))))

(event `S2C_SetIsWorking`
  (params (Unit :type "Actor Object Reference") (ResourceNode :type "Actor Object Reference"))
  (message `/Game/Blueprints/RTS/BPI_RTS_Resource.SetIsWorking` Unit ResourceNode))

(event `Key|RightMouseButton`
  (params (Key :type "Key Structure"))
  (bind (_bblockinghit _binitialoverlap _time _distance _location _impactpoint _normal _impactnormal _physmat _hitactor) (`GameplayStatics.BreakHitResult` (`self.GetHitResultUnderCursorByChannel` "TraceTypeQuery1")))
  (:`Pressed`
    (if (== (`GameplayStatics.GetObjectClass` _hitactor) "/Game/Blueprints/BP_ResourceNode.BP_ResourceNode_C")
      (bind _units (message `/Game/Blueprints/RTS/BPI_RTS_Interface.GrabSelectedUnits` (`self.GetHUD`)))
      (for _array_element _units
        (if (`KismetSystemLibrary.DoesImplementInterface` _array_element "/Game/Blueprints/RTS/BPI_RTS_Resource.BPI_RTS_Resource_C")
          (`self.S2C_SetIsWorking` _array_element _hitactor)))
      (else
        (set `self.RightClickLocation` _location)
        (bind _units_2 (message `/Game/Blueprints/RTS/BPI_RTS_Interface.GrabSelectedUnits` (`self.GetHUD`)))
        (for _array_element_2 _units_2
          (`self.S2C_UnitMoveCommand` _array_element_2 (`self.RightClickLocation`))
          (if (`KismetSystemLibrary.DoesImplementInterface` _array_element_2 "/Game/Blueprints/RTS/BPI_RTS_Resource.BPI_RTS_Resource_C")
            (`self.S2C_SetNotWorking` _array_element_2)))
        (`NiagaraFunctionLibrary.SpawnSystemAtLocation` "/Game/Cursor/FX_Cursor.FX_Cursor" (`self.RightClickLocation`))))))

(event `S2C_SetNotWorking`
  (params (unit :type "Actor Object Reference"))
  (message `/Game/Blueprints/RTS/BPI_RTS_Resource.SetNotWorking` unit))

(event `Key|LeftShift`
  (params (Key :type "Key Structure"))
  (:`Pressed`
    (set `self.LeftShift` true))
  (:`Released`
    (set `self.LeftShift` false)))

(event `S2C_UnitMoveCommand`
  (params (Unit :type "Object Object Reference") (Location :type "Vector Structure"))
  (message `/Game/Blueprints/RTS/BPI_RTS_Interface.UnitMoveCommand` Unit Location))

(event `Key|LeftControl`
  (params (Key :type "Key Structure"))
  (:`Pressed`
    (set `self.LeftCtrl` true))
  (:`Released`
    (set `self.LeftCtrl` false)))

(event `Key|B`
  (params (Key :type "Key Structure"))
  (:`Pressed`
    (`self.StartBuildMode` "/Game/Blueprints/GridByData/DA_RTSBuilding.DA_RTSBuilding")))

(fn `GetResources`
  (returns (Amounts :type Integer))
  (return (`self.ResoureceAmounts`)))

(fn `GetTeam`
  (returns (TeamNumber :type Integer))
  (return 0))

(fn `GrabSelectedUnits`
  (returns (Units :type "Array of Actor Object Reference"))
  (return))

(fn `IsOnMyTeam`
  (params (TeamNumber :type Integer))
  (returns (MyTeam :type Boolean))
  (return (== TeamNumber (`self.Team Number`))))

(fn `SelectBuilding`
  (bind (_bblockinghit _binitialoverlap _time _distance _location _impactpoint _normal _impactnormal _physmat _hitactor) (`GameplayStatics.BreakHitResult` (`self.GetHitResultUnderCursorByChannel` "TraceTypeQuery1")))
  (`self.ClearSelectedBuildings`)
  (if (`KismetMathLibrary.ClassIsChildOf` (`GameplayStatics.GetObjectClass` _hitactor) "/Game/Blueprints/RTS/BP_Building_Base.BP_Building_Base_C")
    (bind _teamnumber (message `/Game/Blueprints/RTS/BPI_RTS_Interface.GetTeam` _hitactor))
    (bind _myteam (message `/Game/Blueprints/RTS/BPI_RTS_Interface.IsOnMyTeam` (`GameplayStatics.GetPlayerController` 0) _teamnumber))
    (if _myteam
      (message `/Game/Blueprints/RTS/BPI_RTS_Interface.SelectedThis_Decal` _hitactor)
      (set `self.SelectedBuilding` _hitactor)
      (return))
    (else
      (return))))

(fn `SetupStart`
  (params (`Player Start Camp` :type "/Game/Blueprints/BP_PlayerStartCamp Object Reference"))
  (set `self.Player Start Camp` `Player Start Camp`)
  (`|ExecutionSequence`
    (:`then_0`
      (`|SpawnActorFromClass` "/Game/Blueprints/RTS/BP_Barrel.BP_Barrel_C" (`SceneComponent.K2_GetComponentToWorld` (`/Game/Blueprints/BP_PlayerStartCamp.StartingBuilding` (`self.Player Start Camp`))) "Undefined" "MultiplyWithRoot" null (`self.Tem Color`) (`self.Team Number`) null))
    (:`then_1`
      (`|SpawnActorFromClass` "/Game/Blueprints/RTS/Units/BP_ResourceUnit.BP_ResourceUnit_C" (`SceneComponent.K2_GetComponentToWorld` (`/Game/Blueprints/BP_PlayerStartCamp.UnitStart1` (`self.Player Start Camp`))) "Undefined" "MultiplyWithRoot" null (`self.Tem Color`) (`self.Team Number`) null))
    (:`then_2`
      (`|SpawnActorFromClass` "/Game/Blueprints/RTS/Units/BP_ResourceUnit.BP_ResourceUnit_C" (`SceneComponent.K2_GetComponentToWorld` (`/Game/Blueprints/BP_PlayerStartCamp.UnitStart2` (`self.Player Start Camp`))) "Undefined" "MultiplyWithRoot" null (`self.Tem Color`) (`self.Team Number`) null))))

(fn `UserConstructionScript`)