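; BP_ResourceUnit is an RTS worker that shuttles resources from a node to its team's drop-off building.
; SetIsWorking stores the node, picks the nearest same-team BP_Building_Base by distance scan and starts moving.
; Collect halts the unit for a timed gather and sends it back, then DropOff credits the team's player controller and returns it to the node.
; S2M multicast events toggle gathering particles and audio, and SetNotWorking cancels the timer.
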(event `S2MDropResource`
  ; Something to do
)

(event `/Game/Blueprints/RTS/BPI_RTSResource.DropOff`
  (if (`self.bIsWorking`)
    (if (`self.bHasResource`)
      (message `/Game/Blueprints/RTS/BPI_RTS_Interface.IncrementResourceAmout` (`GameplayStatics.GetPlayerController` (`self.TeamNumber`)) (`self.ResourceIncresed`))
      (`self.UnitMoveCommand` (`self.K2_GetActorLocation` (`self.ResourceNode`)))
      (set `self.bHasResource` false)
      (`self.S2MDropResource`)
      (`self.UnitMoveCommand` (`self.K2_GetActorLocation` (`self.ResourceNode`)))
      (else
        ; Go back ResourceNode
        (`self.UnitMoveCommand` (`self.K2_GetActorLocation` (`self.ResourceNode`)))))))

(event `S2M_StartCollecting`
  ; MultiCast Start Collecting
  (`ActorComponent.SetActive` (`self.ParticleSystem`) true false)
  (`AudioComponent.Play` (`self.Audio`) 0.0))

(event `S2M_FinishCollecting`
  ; MultiCast Finish Collecting
  (`ActorComponent.SetActive` (`self.ParticleSystem`) false false)
  (`AudioComponent.Stop` (`self.Audio`)))

(event `/Game/Blueprints/RTS/BPI_RTSResource.Collect`
  (if (`self.bIsWorking`)
    (if (`self.bHasResource`)
      ; Head to Command
      (`self.UnitMoveCommand` (`self.K2_GetActorLocation` (`self.DropOffBuilding`)))
      (elif (not (`KismetSystemLibrary.K2_IsValidTimerHandle` (`self.ResourceCollectTime`)))
        ; Stop Movement
        (`self.UnitMoveCommand` (`self.K2_GetActorLocation`))
        ; Collect The Resource
        (`self.S2M_StartCollecting`)
        (bind _returnvalue (`KismetSystemLibrary.K2_SetTimerDelegate` (delegate `ResourceCollecting`) 4.0))
        (set `self.ResourceCollectTime` _returnvalue)))))

(event `ResourceCollecting`
  ; Collect The Resource
  (`KismetSystemLibrary.K2_ClearAndInvalidateTimerHandle` (`self.ResourceCollectTime`))
  (set `self.bHasResource` true)
  (`self.UnitMoveCommand` (`self.K2_GetActorLocation` (`self.DropOffBuilding`)))
  (`self.S2M_FinishCollecting`))

(event `/Game/Blueprints/RTS/BPI_RTSResource.SetNotWorking`
  (set `self.bIsWorking` false)
  (`KismetSystemLibrary.K2_ClearAndInvalidateTimerHandle` (`self.ResourceCollectTime`))
  (`self.S2M_NotWorking`))

(event `S2M_NotWorking`
  (`ActorComponent.SetActive` (`self.ParticleSystem`) false false)
  (`AudioComponent.Stop` (`self.Audio`)))

(event `/Game/Blueprints/RTS/BPI_RTSResource.SetIsWorking`
  (params (ResourceNode :type "Actor Object Reference"))
  (set `self.bIsWorking` true)
  (set `self.ResourceNode` ResourceNode)
  (bind _outactors (`GameplayStatics.GetAllActorsOfClass` "/Game/Blueprints/RTS/BP_Building_Base.BP_Building_Base_C"))
  (for _array_element _outactors
    ; Find Closest Building
    (bind _teamnumber (`/Game/Blueprints/RTS/BPI_RTS_Interface.GetTeam` _array_element))
    (if (== _teamnumber (`self.TeamNumber`))
      (bind _returnvalue (`self.GetDistanceTo` _array_element self))
      (if (< _returnvalue (`self.ClosestDropOffBuildingDistance`))
        (set `self.DropOffBuilding` _array_element)
        (set `self.ClosestDropOffBuildingDistance` _returnvalue))))
  ; Move to Command or Resource
  (if (`self.bHasResource`)
    (`self.UnitMoveCommand` (`self.K2_GetActorLocation` (`self.DropOffBuilding`)))
    (else
      (`self.UnitMoveCommand` (`self.K2_GetActorLocation` (`self.ResourceNode`))))))

(fn `UserConstructionScript`
  (`parent.UserConstructionScript`))