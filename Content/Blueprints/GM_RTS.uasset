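; RTS game mode that gives each joining player a random start camp, a camera pawn and a team.
; The construction script collects all BP_PlayerStartCamp actors into a pool.
; When a player starts, it spawns and possesses a BP_CameraPawn at the chosen camp's CameraStart transform, then sends the controller the camp, team number and indexed team color.
; It then increments the team counter and removes that camp from the pool.
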(event `self.HandleStartingNewPlayer`
  (params (NewPlayer :type "PlayerController Object Reference"))
  (set `self.SelectedStartCamp` (`KismetArrayLibrary.Array_Random` (`self.PlayerStartCamps`)))
  (bind _returnvalue (`|SpawnActorFromClass` "/Game/Blueprints/RTS/BP_CameraPawn.BP_CameraPawn_C" (`SceneComponent.K2_GetComponentToWorld` (`/Game/Blueprints/BP_PlayerStartCamp.CameraStart` (`self.SelectedStartCamp`))) "Undefined" "MultiplyWithRoot" null null))
  (`Controller.Possess` NewPlayer _returnvalue)
  (message `/Game/Blueprints/RTS/BPI_RTS_Interface.SetupPlayerStart` NewPlayer (`self.SelectedStartCamp`) (`self.TeamNumber`) (`|GetArrayItem` (`self.TeamColor`) (`self.TeamNumber`)))
  (`/Engine/EditorBlueprintResources/StandardMacros.IncrementInt` (`self.TeamNumber`)
    (:`  `
      (`KismetArrayLibrary.Array_RemoveItem` (`self.PlayerStartCamps`) (`self.SelectedStartCamp`)))))

(fn `UserConstructionScript`
  (locals (NewLocalVar :type "Array of /Game/Blueprints/BP_PlayerStartCamp Object Reference"))
  (bind _outactors (`GameplayStatics.GetAllActorsOfClass` "/Game/Blueprints/BP_PlayerStartCamp.BP_PlayerStartCamp_C"))
  (set `self.PlayerStartCamps` _outactors))