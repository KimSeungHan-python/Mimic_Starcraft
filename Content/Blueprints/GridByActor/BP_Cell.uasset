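; BP_Cell is a single cell actor for an actor-based grid, showing placement feedback on its Plane mesh.
; SetCellState stores the state and swaps the material: white for idle, green for can place, red for both cannot place and selected.
; SetOccupied only stores the occupancy flag, without changing the visual.
; The cell has no event or construction logic of its own.
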(fn `SetCellState`
  (params (CurrentState :type "/Game/Blueprints/GridByActor/E_CellState Enum" :default "NewEnumerator0"))
  (bind _output_get (set `self.CurrentState` CurrentState))
  (switch `/Game/Blueprints/GridByActor/E_CellState` _output_get
    (:`NewEnumerator0`
      (`PrimitiveComponent.SetMaterial` (`self.Plane`) 0 "/Game/Blueprints/GridByActor/MI_CellWhite.MI_CellWhite"))
    (:`NewEnumerator1`
      (`PrimitiveComponent.SetMaterial` (`self.Plane`) 0 "/Game/Blueprints/GridByActor/MI_CellGreen.MI_CellGreen"))
    (:`NewEnumerator2`
      (`PrimitiveComponent.SetMaterial` (`self.Plane`) 0 "/Game/Blueprints/GridByActor/MI_CellRed.MI_CellRed"))
    (:`NewEnumerator3`
      (`PrimitiveComponent.SetMaterial` (`self.Plane`) 0 "/Game/Blueprints/GridByActor/MI_CellRed.MI_CellRed"))))

(fn `SetOccupied`
  (params (bIsOccupied :type Boolean))
  (set `self.bIsOccupied` bIsOccupied))

(fn `UserConstructionScript`)