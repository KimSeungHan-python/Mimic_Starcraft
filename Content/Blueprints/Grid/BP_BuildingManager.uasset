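; Grid-based building manager that handles placing, rotating, selecting and deleting buildings through an idle, placing and selecting state machine.
; BeginPlay spawns a centered grid of BP_Cell actors, with helpers converting between world and grid coordinates.
; Mouse traces snap the held building to cells and pick existing buildings, while footprints drive cell occupancy.
; The footprint validation and highlight logic is disconnected from its function entry, so it never runs.
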(event `self.ReceiveBeginPlay`
  (`self.InitializeGrid`))

(event `self.ReceiveTick`
  (params (DeltaSeconds :type "Float (single-precision)"))
  (`self.HeldBuilding`
    (:`then`
      (switch `/Game/Blueprints/Grid/E_GameState` (`self.CurrentGameState`)
        (:`NewEnumerator1`
          (`self.UpdateCursorBuildingPosition`))))
    (:`else`)))

(fn `CancelCurrentAction`
  (switch `/Game/Blueprints/Grid/E_GameState` (`self.CurrentGameState`)
    (:`NewEnumerator1`
      (bind _heldbuilding (`self.HeldBuilding`)
        (:`then`
          ; 추후 건물파괴
          (`self.K2_DestroyActor` _heldbuilding)
          (set `self.HeldBuilding` null)
          (`self.ClearHighlight`))
        (:`else`)))
    (:`NewEnumerator2`
      (bind _selectedbuilding (`self.SelectedBuilding`)
        (:`then`
          (`/Game/Blueprints/Grid/BP_Building.SetSelected` _selectedbuilding false)
          (set `self.SelectedBuilding` null))
        (:`else`))))
  (set `self.CurrentGameState` "NewEnumerator0"))

(fn `ClearHighlight`
  (for _array_element (`self.PreviewHighlightGridCell`)
    (`/Game/Blueprints/Grid/BP_Cell.SetCellState` _array_element "NewEnumerator0"))
  (`KismetArrayLibrary.Array_Clear` (`self.PreviewHighlightGridCell`)))

(fn `CommitBuildingToGrid`
  (locals (CurrentCell :type "/Game/Blueprints/Grid/BP_Cell Object Reference") (Coord :type "IntPoint Structure"))
  (bind _selectedbuilding (`self.SelectedBuilding`)
    (:`then`
      (set `local.CurrentCell` (`self.GetCellAtWorldPosition` (`self.K2_GetActorLocation` _selectedbuilding)))
      (for _array_element (`/Game/Blueprints/Grid/BP_Building.GetFootPrint` (`self.HeldBuilding`))
        (bind _output_get (set `local.Coord` (+ _array_element (`/Game/Blueprints/Grid/BP_Cell.GridCoord` (`local.CurrentCell`)))))
        (if (`self.IsValidCoordinate` _output_get)
          (`/Game/Blueprints/Grid/BP_Cell.SetOccupied` (`self.GetCellAtGridCoordinate` (`local.Coord`)) true)))
      (`self.ClearHighlight`)
      (`/Game/Blueprints/Grid/BP_Building.SetBlueBuilding` (`self.HeldBuilding`))
      (set `self.HeldBuilding` null)
      (set `self.CurrentGameState` "NewEnumerator0"))
    (:`else`)))

(fn `DeleteSelectBuilding`
  (locals (Cell :type "/Game/Blueprints/Grid/BP_Cell Object Reference"))
  (bind _selectedbuilding (`self.SelectedBuilding`)
    (:`then`
      (set `local.Cell` (`self.GetCellAtWorldPosition` (`self.K2_GetActorLocation` _selectedbuilding)))
      (for _array_element (`/Game/Blueprints/Grid/BP_Building.GetFootPrint` (`self.SelectedBuilding`))
        (`/Game/Blueprints/Grid/BP_Cell.SetOccupied` (`self.GetCellAtGridCoordinate` (+ _array_element (`/Game/Blueprints/Grid/BP_Cell.GridCoord` (`local.Cell`)))) false))
      (`self.K2_DestroyActor` (`self.SelectedBuilding`))
      (set `self.SelectedBuilding` null)
      (set `self.CurrentGameState` "NewEnumerator0"))
    (:`else`)))

(fn `DeselectBuilding`
  (bind _selectedbuilding (`self.SelectedBuilding`)
    (:`then`
      (`/Game/Blueprints/Grid/BP_Building.SetSelected` _selectedbuilding false)
      (set `self.SelectedBuilding` null)
      (set `self.CurrentGameState` "NewEnumerator0"))
    (:`else`)))

(fn `GetCellAtGridCoordinate`
  (params (`Grid Coord` :type "IntPoint Structure"))
  (returns (Cell :type "/Game/Blueprints/Grid/BP_Cell Object Reference"))
  (locals (Index :type Integer))
  (bind (_x _y) (break `IntPoint` `Grid Coord`))
  (if (`self.IsValidCoordinate` `Grid Coord`)
    (set `local.Index` (+ _x (* _y (`self.Width`))))
    (if (and (>= (`local.Index`) 0) (<= (`local.Index`) (`KismetArrayLibrary.Array_Length` (`self.GridCell`))))
      (return (`|GetArrayItem` (`self.GridCell`) (`local.Index`))))))

(fn `GetCellAtWorldPosition`
  (params (NewParam :type "Vector Structure"))
  (returns (Cell :type "/Game/Blueprints/Grid/BP_Cell Object Reference"))
  (return (`self.GetCellAtGridCoordinate` (`self.WorldToGrid` NewParam))))

(fn `GetGridStartLocation`
  (returns (ReturnValue :type "Vector Structure"))
  (return (- (`self.K2_GetActorLocation`) (`KismetMathLibrary.MakeVector` (/ (* (`self.Width`) (`self.CellSize`)) 2.0) (/ (* (`self.Height`) (`self.CellSize`)) 2.0)))))

(fn `GridToWorld`
  (params (Grid :type "IntPoint Structure"))
  (returns (ReturnValue :type "Vector Structure"))
  (return (+ (`self.GetGridStartLocation`) (`KismetMathLibrary.MakeVector` (+ (* Grid_X (`self.CellSize`)) (/ (`self.CellSize`) 2.0)) (+ (* Grid_Y (`self.CellSize`)) (/ (`self.CellSize`) 2.0))))))

(fn `HandleDelete`
  (switch `/Game/Blueprints/Grid/E_GameState` (`self.CurrentGameState`)
    (:`NewEnumerator2`
      (`self.DeleteSelectBuilding`))))

(fn `HandleLeftClick`
  (bind (_locationx _locationy) (`PlayerController.GetMousePosition` (`GameplayStatics.GetPlayerController` 0)))
  (bind (_worldposition _worlddirection) (`GameplayStatics.DeprojectScreenToWorld` (`GameplayStatics.GetPlayerController` 0) (`KismetMathLibrary.MakeVector2D` _locationx _locationy)))
  (switch `/Game/Blueprints/Grid/E_GameState` (`self.CurrentGameState`)
    (:`NewEnumerator0`
      (bind _outhit (`KismetSystemLibrary.LineTraceSingle` _worldposition (+ _worldposition (* _worlddirection 50000.0)) "TraceTypeQuery1"))
      (bind _asbp_building (cast `/Game/Blueprints/Grid/BP_Building` (`.HitActor` (`GameplayStatics.BreakHitResult` _outhit))))
      (`self.SelectBuildingOnGrid` _asbp_building))
    (:`NewEnumerator1`
      (bind _heldbuilding (`self.HeldBuilding`)
        (:`then`
          (bind _cell (`self.GetCellAtWorldPosition` (`self.K2_GetActorLocation` _heldbuilding)))
          (`/Engine/EditorBlueprintResources/StandardMacros.IsValid` _cell
            (:`Is Valid`
              (bind _bcanplace1 (`self.ValidateAndHighLightPlacement` (`/Game/Blueprints/Grid/BP_Cell.GridCoord` _cell) (`/Game/Blueprints/Grid/BP_Building.GetFootPrint` (`self.HeldBuilding`))))
              (if _bcanplace1
                (`self.CommitBuildingToGrid`)))))
        (:`else`)))))

(fn `HandleRightClick`
  (`self.CancelCurrentAction`))

(fn `HandleRotateKey`
  (switch `/Game/Blueprints/Grid/E_GameState` (`self.CurrentGameState`)
    (:`NewEnumerator1`
      (`self.RotateHeldBuilding`))))

(fn `InitializeGrid`
  (locals (Y :type Integer) (X :type Integer))
  (for _index (range (`self.Height`))
    (set `local.Y` _index)
    (for _index_2 (range (`self.Width`))
      (set `local.X` _index_2)
      (bind _returnvalue (`|SpawnActorFromClass` "/Game/Blueprints/Grid/BP_Cell.BP_Cell_C" (`KismetMathLibrary.MakeTransform` (`self.GridToWorld` (make `IntPoint` (`local.X`) (`local.Y`)))) "Undefined" "MultiplyWithRoot" null null))
      (set `/Game/Blueprints/Grid/BP_Cell.GridCoord` (make `IntPoint` (`local.X`) (`local.Y`)) _returnvalue)
      (`KismetArrayLibrary.Array_Add` (`self.GridCell`) _returnvalue))))

(fn `IsValidCoordinate`
  (params (`Grid Coord` :type "IntPoint Structure"))
  (returns (NewParam :type Boolean))
  (bind (_grid_coord_x _grid_coord_y) (break `IntPoint` (`local.Grid Coord`)))
  (return (and (>= `Grid Coord_X` 0) (>= `Grid Coord_Y` 0) (< _grid_coord_x (`self.Width`)) (< _grid_coord_y (`self.Height`)))))

(fn `RotateHeldBuilding`
  (bind (_returnvalue_roll _returnvalue_pitch _returnvalue_yaw) (`KismetMathLibrary.BreakRotator` (`self.K2_GetActorRotation` (`self.HeldBuilding`))))
  (bind _heldbuilding (`self.HeldBuilding`)
    (:`then`
      (set `/Game/Blueprints/Grid/BP_Building.CurrentRotation` (mod (+ (`/Game/Blueprints/Grid/BP_Building.CurrentRotation` _heldbuilding) 90) 360) _heldbuilding)
      (`self.K2_SetActorRotation` (`KismetMathLibrary.MakeRotator` _returnvalue_roll _returnvalue_pitch (+ _returnvalue_yaw 90.0)))
      (`self.ValidateAndHighLightPlacement` (`/Game/Blueprints/Grid/BP_Cell.GridCoord` (`self.GetCellAtWorldPosition` (`self.K2_GetActorLocation` (`self.HeldBuilding`)))) (`/Game/Blueprints/Grid/BP_Building.GetFootPrint` (`self.HeldBuilding`))))
    (:`else`)))

(fn `SelectBuildingOnGrid`
  (params (TargetBuilding :type "/Game/Blueprints/Grid/BP_Building Object Reference"))
  (`/Engine/EditorBlueprintResources/StandardMacros.IsValid` TargetBuilding
    (:`Is Valid`
      (`self.CancelCurrentAction`)
      (bind _output_get (set `self.SelectedBuilding` TargetBuilding))
      (`/Game/Blueprints/Grid/BP_Building.SetSelected` _output_get true)
      (set `self.CurrentGameState` "NewEnumerator2"))))

(fn `SpawnAndAttachBuilding`
  (params (Class :type "/Game/Blueprints/Grid/BP_Building Class Reference") (BuildingType :type "/Game/Blueprints/Grid/E_BuildingType Enum" :default "NewEnumerator0"))
  (locals (Type :type "/Game/Blueprints/Grid/E_BuildingType Enum" :default "NewEnumerator0"))
  (set `local.Type` BuildingType)
  (`self.CancelCurrentAction`)
  (bind _returnvalue (`|SpawnActorFromClass` Class (`KismetMathLibrary.MakeTransform` (0.0 0.0 0.0)) "Undefined" "MultiplyWithRoot" null null))
  (bind _output_get (set `self.HeldBuilding` _returnvalue))
  (set `/Game/Blueprints/Grid/BP_Building.BuildingType` (`local.Type`) _output_get)
  (set `/Game/Blueprints/Grid/BP_Building.CurrentRotation` 0 _output_get)
  (set `self.CurrentGameState` "NewEnumerator1")
  (`self.UpdateCursorBuildingPosition`))

(fn `UpdateCursorBuildingPosition`
  (locals (HitCell :type "/Game/Blueprints/Grid/BP_Cell Object Reference"))
  (bind (_locationx _locationy) (`PlayerController.GetMousePosition` (`GameplayStatics.GetPlayerController` 0)))
  (bind (_worldposition _worlddirection) (`GameplayStatics.DeprojectScreenToWorld` (`GameplayStatics.GetPlayerController` 0) (`KismetMathLibrary.MakeVector2D` _locationx _locationy)))
  (`self.HeldBuilding`
    (:`then`
      (switch `/Game/Blueprints/Grid/E_GameState` (`self.CurrentGameState`)
        (:`NewEnumerator1`
          (bind _outhit (`KismetSystemLibrary.LineTraceSingle` _worldposition (+ _worldposition (* _worlddirection 50000.0)) "TraceTypeQuery1"))
          (bind _cell (`self.GetCellAtWorldPosition` (`.Location` (`GameplayStatics.BreakHitResult` _outhit))))
          (`/Engine/EditorBlueprintResources/StandardMacros.IsValid` _cell
            (:`Is Valid`
              (bind _output_get (set `local.HitCell` _cell))
              (`self.K2_SetActorLocation` (`self.HeldBuilding`) (`self.GridToWorld` (`/Game/Blueprints/Grid/BP_Cell.GridCoord` _output_get)) false false)
              (`self.ValidateAndHighLightPlacement` (`/Game/Blueprints/Grid/BP_Cell.GridCoord` (`local.HitCell`)) (`/Game/Blueprints/Grid/BP_Building.GetFootPrint` (`self.HeldBuilding`))))))))
    (:`else`)))

(fn `UserConstructionScript`)

(fn `ValidateAndHighLightPlacement`
  (params (GridOrigin :type "IntPoint Structure") (FootPrint :type "Array of IntPoint Structure"))
  (returns (bCanPlace1 :type Boolean))
  (locals (Origin :type "IntPoint Structure") (PrintFoot :type "Array of IntPoint Structure") (bCanPlace :type Boolean) (Coord :type "IntPoint Structure") (CellToHighlight :type "Array of /Game/Blueprints/Grid/BP_Cell Object Reference") (Highlight :type "/Game/Blueprints/Grid/E_CellState Enum"))
  (set `local.Origin` GridOrigin)
  (set `local.PrintFoot` FootPrint))

(fn `WorldToGrid`
  (params (NewParam :type "Vector Structure"))
  (returns (IntPoint :type "IntPoint Structure"))
  (bind (_returnvalue_x _returnvalue_y) (`KismetMathLibrary.BreakVector` (- NewParam (`self.GetGridStartLocation`))))
  (return (make `IntPoint` (`KismetMathLibrary.FFloor` (/ _returnvalue_x (`self.CellSize`))) (`KismetMathLibrary.FFloor` (/ _returnvalue_y (`self.CellSize`))))))