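; BP_Building is a grid building actor that starts with a ghost material and reports the footprint it occupies.
; On BeginPlay it constructs an O_ShapeHelper object, which supplies base footprints for the vertical, horizontal and 2x2 square building types.
; GetFootPrint picks the shape by BuildingType, then rotates it repeatedly in 90-degree steps based on CurrentRotation.
; Separate functions switch the mesh to blue, or toggle orange and blue for selection.
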(event `self.ReceiveBeginPlay`
  (bind _returnvalue (`|GenericCreateObject` "/Game/Blueprints/Grid/O_ShapeHelper.O_ShapeHelper_C"))
  (set `self.ShapedHelper` _returnvalue)
  (`PrimitiveComponent.SetMaterial` (`self.StaticMesh`) 0 "/Game/Blueprints/Grid/MI_BuildingGhost.MI_BuildingGhost"))

(fn `GetFootPrint`
  (returns (RotationFootprint1 :type "Array of IntPoint Structure"))
  (locals (BaseFootprint :type "Array of IntPoint Structure") (RotationFootprint :type "Array of IntPoint Structure"))
  (switch `/Game/Blueprints/Grid/E_BuildingType` (`self.BuildingType`)
    (:`NewEnumerator0`
      (set `local.BaseFootprint` (`/Game/Blueprints/Grid/O_ShapeHelper.GetVerticle` (`self.ShapedHelper`))))
    (:`NewEnumerator1`
      (set `local.BaseFootprint` (`/Game/Blueprints/Grid/O_ShapeHelper.GetHorizontal` (`self.ShapedHelper`))))
    (:`NewEnumerator2`
      (set `local.BaseFootprint` (`/Game/Blueprints/Grid/O_ShapeHelper.GetSquare2*2` (`self.ShapedHelper`)))))
  (set `local.RotationFootprint` (`local.BaseFootprint`))
  (for _ (range (+ (/ (`self.CurrentRotation`) 90) 1))
    (set `local.RotationFootprint` (`/Game/Blueprints/Grid/O_ShapeHelper.GetRotate` (`self.ShapedHelper`) (`local.RotationFootprint`))))
  (return (`local.RotationFootprint`)))

(fn `SetBlueBuilding`
  (`PrimitiveComponent.SetMaterial` (`self.StaticMesh`) 0 "/Game/Blueprints/Grid/MI_BuildingBlue.MI_BuildingBlue"))

(fn `SetSelected`
  (params (bIsSelected :type Boolean))
  (if bIsSelected
    (`PrimitiveComponent.SetMaterial` (`self.StaticMesh`) 0 "/Game/Blueprints/Grid/MI_BuildingOrange.MI_BuildingOrange")
    (else
      (`PrimitiveComponent.SetMaterial` (`self.StaticMesh`) 0 "/Game/Blueprints/Grid/MI_BuildingBlue.MI_BuildingBlue"))))

(fn `UserConstructionScript`)