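; O_ShapeHelper is a grid helper that supplies cell footprints for shapes as arrays of IntPoint offsets.
; GetShapeFootprint picks a two-cell line or 2x2 square by shape type, with the Vertical case returning the horizontal offsets and Horizontal the vertical ones.
; GetRotate turns any footprint 90 degrees about the origin by mapping each (X, Y) to (-Y, X).
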(fn `GetHorizontal`
  (returns (Array :type "Array of IntPoint Structure"))
  (return (`|MakeArray` (make `IntPoint` 0) (make `IntPoint` 1))))

(fn `GetRotate`
  (params (NewParam :type "Array of IntPoint Structure"))
  (returns (NewParam1 :type "Array of IntPoint Structure"))
  (locals (Out :type "Array of IntPoint Structure"))
  (for _array_element NewParam
    (bind (_x _y) (break `IntPoint` _array_element))
    (`KismetArrayLibrary.Array_Add` (`local.Out`) (make `IntPoint` (* _y -1) _x)))
  (return (`local.Out`)))

(fn `GetShapeFootprint`
  (returns (Array :type "Array of IntPoint Structure"))
  (switch `/Game/Blueprints/Grid/E_BuildingType` "NewEnumerator0"
    (:`NewEnumerator0`
      (return (`self.GetHorizontal`)))
    (:`NewEnumerator1`
      (return (`self.GetVerticle`)))
    (:`NewEnumerator2`
      (return (`self.GetSquare2*2`)))))

(fn `GetSquare2*2`
  (returns (Array :type "Array of IntPoint Structure"))
  (return (`|MakeArray` (make `IntPoint` 0) (make `IntPoint` 1) (make `IntPoint` 0 1) (make `IntPoint` 1 1))))

(fn `GetVerticle`
  (returns (Array :type "Array of IntPoint Structure"))
  (return (`|MakeArray` (make `IntPoint` 0) (make `IntPoint` 0 1))))